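; BP_CUBE_GAnerate is a grid generator that lays out blocks on an X by Y plane with Padding spacing.
; Its construction script adds static mesh components as a preview, storing them in PreviwArray and looping one index further per axis than the runtime grid.
; BeginPlay destroys the preview components and spawns BP_Blocks_Child actors offset from the actor's X and Y location, at world Z zero.
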(event `self.ReceiveBeginPlay`
  (bind (_returnvalue_x _returnvalue_y) (`KismetMathLibrary.BreakVector` (`self.K2_GetActorLocation`)))
  (for _array_element (`self.PreviwArray`)
    (`ActorComponent.K2_DestroyComponent` _array_element))
  (for _index (range (`self.x`))
    (for _index_2 (range (`self.y`))
      (`|SpawnActorFromClass` "/Game/BP_Blocks_Child.BP_Blocks_Child_C" (`KismetMathLibrary.MakeTransform` (`KismetMathLibrary.MakeVector` (+ _returnvalue_x (`KismetMathLibrary.Conv_IntToDouble` (* _index (`self.padding`)))) (+ _returnvalue_y (`KismetMathLibrary.Conv_IntToDouble` (* _index_2 (`self.padding`)))))) "Undefined" "OverrideRootScale" null null))))

(fn `UserConstructionScript`
  (for _index (range (+ (`self.x`) 1))
    (for _index_2 (range (+ (`self.y`) 1))
      (bind _returnvalue (`AddComponent|NODE_AddStaticMeshComponent-0` :`RelativeTransform` (`KismetMathLibrary.MakeTransform` (`KismetMathLibrary.MakeVector` (`KismetMathLibrary.Conv_IntToDouble` (* _index (`self.padding`))) (`KismetMathLibrary.Conv_IntToDouble` (* _index_2 (`self.padding`)))))))
      (`KismetArrayLibrary.Array_Add` (`self.PreviwArray`) _returnvalue))))